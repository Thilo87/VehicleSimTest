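; Style 1 traffic light Blueprint that shows the current light phase by swapping materials on the lamp slots of its static mesh.
; The parent's construction script runs first, then the starting phase is applied to the mesh.
; Each phase change event blanks all three lamps to black, then lights red, amber or green, with red and amber together for the Red Amber phase.
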(event EventOnTrafficLightPhaseChanged
  (params (NewTrafficLightPhase :type ETrafficLightPhase%20Enum :default "Red"))
  (CallFunction|ChangePhaseColor NewTrafficLightPhase))

(fn ConstructionScript
  (|CallParentFunction)
  (CallFunction|ResetColors)
  (CallFunction|ChangePhaseColor (Variables|Default|GetStartingPhase)))

(fn ResetColors
  (Rendering|Material|SetMaterial (Variables|Default|GetStaticMesh) 1 (Variables|Default|GetBlackMaterial))
  (Rendering|Material|SetMaterial (Variables|Default|GetStaticMesh) 2 (Variables|Default|GetBlackMaterial))
  (Rendering|Material|SetMaterial (Variables|Default|GetStaticMesh) 3 (Variables|Default|GetBlackMaterial)))

(fn ChangePhaseColor
  (params (Phase :type ETrafficLightPhase%20Enum :default "Red"))
  (CallFunction|ResetColors)
  (switch Utilities|FlowControl|Switch|SwitchonETrafficLightPhase Phase
    (:Red
      (Rendering|Material|SetMaterial (Variables|Default|GetStaticMesh) 1 (Variables|Default|GetRedMaterial)))
    (:RedAmber
      (Rendering|Material|SetMaterial (Variables|Default|GetStaticMesh) 1 (Variables|Default|GetRedMaterial))
      (Rendering|Material|SetMaterial (Variables|Default|GetStaticMesh) 2 (Variables|Default|GetAmberMaterial)))
    (:Green
      (Rendering|Material|SetMaterial (Variables|Default|GetStaticMesh) 3 (Variables|Default|GetGreenMaterial)))
    (:Amber
      (Rendering|Material|SetMaterial (Variables|Default|GetStaticMesh) 2 (Variables|Default|GetAmberMaterial)))))