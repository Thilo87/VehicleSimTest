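; Speed zone actor for traffic regulation, pairing a box volume (Zone) with a SpeedSign component.
; The construction script offsets Zone by its extents along -X and +Z, so it extends backward and upward from its reference point.
; It also sets the sign's Y to the negative box Y extent, keeping it aligned with the side as the box is resized.
; The event graph holds no active logic.
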(event EventBeginPlay)

(event Collision|EventActorBeginOverlap
  (params (OtherActor :type Actor%20Object%20Reference)))

(event EventTick
  (params (DeltaSeconds :type Float%20%28single-precision%29)))

(fn ConstructionScript
  (bind _speedsign (Variables|Default|GetSpeedSign))
  (bind _zone (Variables|Default|GetZone))
  (bind _boxextent (Variables|/Script/Engine.BoxComponent|GetBoxExtent _zone))
  (bind _relativelocation (Variables|/Script/Engine.SceneComponent|GetRelativeLocation _speedsign))
  (Utilities|FlowControl|Sequence
    (:then_0
      (Transformation|SetRelativeLocation _speedsign (Math|Vector|MakeVector (.x _relativelocation) (* (.y (Variables|/Script/Engine.BoxComponent|GetBoxExtent (Variables|Default|GetZone))) -1.0) (.z _relativelocation)) false false))
    (:then_1
      (Transformation|SetRelativeLocation _zone (Math|Vector|MakeVector (* (.x _boxextent) -1.0) 0.0 (.z _boxextent)) false false))))